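; BP_Character1 is a character Blueprint that supports swapping the controlled character in place through two possession-handoff events.
; UpdateCharacterBeforeUnpossess hides the mesh and disables mesh and capsule collision.
; UpdateCharAfterPosses shows the mesh, teleports to the old character's transform, then waits one tick before restoring collision.
; A CurvedNoise effect spawn is left unconnected and never runs.
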(event Custom|UpdateCharAfterPosses
  (params (OldCharacter :type BP%20Character%201%20Object%20Reference))
  (bind _returnvalue (Transformation|GetActorTransform OldCharacter))
  (Rendering|SetVisibility (Variables|Character|GetMesh) true true)
  (Transformation|SetActorLocationAndRotation (.location _returnvalue) (.rotation _returnvalue) false true)
  (Utilities|FlowControl|DelayUntilNextTick)
  (Collision|SetCollisionEnabled (Variables|Collision|GetCapsuleComponent) "QueryAndPhysics")
  (Collision|SetCollisionEnabled (Variables|Character|GetMesh) "QueryAndPhysics"))

(event Custom|UpdateCharacterBeforeUnpossess
  (bind _mesh (Variables|Character|GetMesh))
  (Rendering|SetVisibility _mesh false true)
  (Collision|SetCollisionEnabled _mesh "NoCollision")
  (Collision|SetCollisionEnabled (Variables|Collision|GetCapsuleComponent) "NoCollision"))

(event EventBeginPlay)

(event Collision|EventActorBeginOverlap
  (params (OtherActor :type Actor%20Object%20Reference)))

(event EventTick
  (params (DeltaSeconds :type Float%20%28single-precision%29)))

(fn ConstructionScript)