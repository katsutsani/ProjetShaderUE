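; Character Blueprint that triggers a timed smoke-and-aura shader effect when the A key is pressed.
; Activation applies a smoke overlay material to the mesh, shows the aura and screen aura components, and plays an attached sound.
; The sound's finish event acts as the timer, clearing the effect and resetting the IsActivated and IsVisible flags.
; Pressing A during the effect only sets IsVisible back to true.
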(event Custom|Onfinished
  (Rendering|Material|SetOverlayMaterial (Variables|Character|GetMesh) 0 :!class /Script/Engine.MeshComponent)
  (Rendering|SetVisibility (Variables|Default|GetN_AuraM) false false)
  (Rendering|SetVisibility (Variables|Default|GetAuraScreen) false false)
  (Variables|Default|SetIsActivated false)
  (Variables|Default|SetIsVisible true))

(event EventBeginPlay
  (|CallParentFunction) ; This node is disabled and will not be called.\nDrag off pins to build functionality.
)

(event Collision|EventActorBeginOverlap
  (params (OtherActor :type Actor%20Object%20Reference))
  (|CallParentFunction OtherActor) ; This node is disabled and will not be called.\nDrag off pins to build functionality.
)

(event Input|KeyboardEvents|A
  (params (Key :type Key%20Structure :default "None"))
  (bind _mesh (Variables|Character|GetMesh))
  (:Pressed
    (if (Variables|Default|GetIsActivated)
      (Variables|Default|SetIsVisible true)
      (else
        (Variables|Default|SetIsActivated true)
        (Variables|Default|SetIsVisible false)
        (Rendering|Material|SetOverlayMaterial _mesh "/Game/ContentManu/VIsualEffects/Material/M_SmokeM.M_SmokeM" :!class /Script/Engine.MeshComponent)
        (Rendering|SetVisibility (Variables|Default|GetN_AuraM) true false)
        (Rendering|SetVisibility (Variables|Default|GetAuraScreen) true false)
        (bind _returnvalue (Audio|SpawnSoundAttached "/Game/ContentManu/SFX/SW_ShadersSound_M.SW_ShadersSound_M" _mesh "None" "0, 0, 0" "0, 0, 0" "KeepRelativeOffset" true 0.1 1.0 0.0 0 0))
        (EventDispatchers|BindEventtoOnAudioFinished _returnvalue (delegate Custom|Onfinished))))))

(fn ConstructionScript
  (|CallParentFunction))