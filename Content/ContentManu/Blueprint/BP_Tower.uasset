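; BP_Tower is a tower actor that shoots at nearby pawns and shows its health on a UI_Ennemie bar.
; Tick runs a 0.2s Delay, then SphereTrace picks the last in-radius pawn, ignoring one BP_Ennemie, and BP_BulletTower spawns aimed at it.
; Tick also updates the bar, spawns BP_TowerExplosion every tick while life is above zero but at most half, and calls SetLifeSpan(0) at zero.
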(event Custom|DestroyTower
  (Game|SpawnActorfromClass "/Game/Emile/MasterField/BP_TowerExplosion.BP_TowerExplosion_C" (Math|Transform|MakeTransform (Transformation|GetWorldLocation (Variables|Default|GetArrow)) "0, 0, 0" "8.000000,8.000000,8.000000") "Undefined" "MultiplyWithRoot" 0 0))

(event EventTick
  (params (DeltaSeconds :type Float%20%28single-precision%29))
  (bind _arrow (Variables|Default|GetArrow))
  (bind _currentlife (Variables|Default|GetCurrentLife))
  (bind _maxlife (Variables|Default|GetMaxLife))
  (bind _returnvalue (Transformation|GetWorldTransform _arrow))
  (Utilities|FlowControl|Sequence
    (:then_0
      (Utilities|FlowControl|Delay 0.2)
      (bind _hit_actor (CallFunction|SphereTrace))
      (Utilities|IsValid _hit_actor
        (:Is%20Valid
          (Game|SpawnActorfromClass "/Game/ContentManu/Blueprint/BP_BulletTower.BP_BulletTower_C" (Math|Transform|MakeTransform (.location _returnvalue) (Math|Rotator|FindLookatRotation (.location _returnvalue) (Transformation|GetActorLocation _hit_actor)) "1.000000,1.000000,1.000000") "AdjustIfPossibleButAlwaysSpawn" "MultiplyWithRoot" 0 0))))
    (:then_1
      (bind _asui_ennemie (Utilities|Casting|CastToUI_Ennemie (UserInterface|GetWidget (Variables|Default|GetUIBarreDePV))))
      (Default|HPFunction _asui_ennemie _currentlife _maxlife)
      (if (<= _currentlife (/ _maxlife 2.0))
        (if (<= _currentlife 0.0)
          (Actor|SetLifeSpan 0.0)
          (else
            (CallFunction|DestroyTower)))))))

(fn ConstructionScript)

(fn SphereTrace
  (bind _returnvalue (Transformation|GetActorLocation))
  (bind _returnvalue_2 (Actor|GetActorOfClass "/Game/ContentManu/Blueprint/BP_Ennemie.BP_Ennemie_C"))
  (bind _outhits (Collision|MultiSphereTraceForObjects _returnvalue _returnvalue (Variables|Default|GetRadius) (Utilities|Array|MakeArray "ObjectTypeQuery3") false (Utilities|Array|MakeArray _returnvalue_2) "Persistent"))
  (for _array_element _outhits
    (if (< (Math|Vector|Distance(Vector) (Transformation|GetActorLocation (.hitactor _array_element)) (Transformation|GetActorLocation)) (Variables|Default|GetRadius))
      (LocalVariables|SetActorHit (.hitactor _array_element))))
  (return (LocalVariables|GetActorHit)))