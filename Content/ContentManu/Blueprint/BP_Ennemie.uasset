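; BP_Ennemie is an AI enemy that pushes its life to a widget health bar every Tick and destroys itself at zero.
; PawnSensing sets the blackboard key HasSeenPlayer according to whether the sighted BP_Character_M is visible.
; AttackPlayer sphere-traces forward for pawns, then plays a montage, damages a hit BP_Character1 and launches it upward with an X-only impulse based on the victim's facing.
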(event OnSeePawn(PawnSensing)
  (params (Pawn :type Pawn%20Object%20Reference))
  (bind _asbp_character_m (Utilities|Casting|CastToBP_Character_M Pawn))
  (if (Variables|/Game/ContentManu/Blueprint/BP_Character_M.BP_Character_M_C|GetIsVisible _asbp_character_m)
    (Actor|GetAllActorsOfClass "/Game/ThirdParty/Stylized_VFX_StPack/Blueprints/UPDATE_1_4/BP_Character.BP_Character_C")
    (AI|Components|Blackboard|SetValueasBool (AI|GetBlackboard (AI|GetAIController self)) (Utilities|Name|MakeLiteralName "HasSeenPlayer") true)
    (else
      (Actor|GetAllActorsOfClass "/Game/ThirdParty/Stylized_VFX_StPack/Blueprints/UPDATE_1_4/BP_Character.BP_Character_C")
      (AI|Components|Blackboard|SetValueasBool (AI|GetBlackboard (AI|GetAIController self)) (Utilities|Name|MakeLiteralName "HasSeenPlayer") false))))

(event Custom|AttackPlayer
  (bind _returnvalue (Transformation|GetActorLocation))
  (bind (_outhit _returnvalue_2) (Collision|SphereTraceForObjects _returnvalue (+ _returnvalue (* (Math|Vector|GetForwardVector (Transformation|GetActorRotation)) 2.5e+02)) (Variables|Default|GetRange) (Utilities|Array|MakeArray "ObjectTypeQuery3") false 0 "ForDuration"))
  (if _returnvalue_2
    (bind _asbp_character_1 (Utilities|Casting|CastToBP_Character1 (.HitActor (Collision|BreakHitResult _outhit))))
    (Animation|PlayAnimMontage "/Game/ContentManu/Blueprint/Anim_Attack1_Montage.Anim_Attack1_Montage" 1.0 "None")
    (Default|Health _asbp_character_1 (Variables|Default|GetDmg))
    (Physics|AddImpulse (Variables|/Script/Engine.Character|GetCharacterMovement _asbp_character_1) (Math|Vector|MakeVector (* (.x (Math|Vector|GetForwardVector (Transformation|GetActorRotation _asbp_character_1))) -5e+02) 0.0 3e+02) true)))

(event EventTick
  (params (DeltaSeconds :type Float%20%28single-precision%29))
  (bind _asui_ennemie (Utilities|Casting|CastToUI_Ennemie (UserInterface|GetWidget (Variables|Default|GetHealthBar))))
  (Default|HPFunction _asui_ennemie (Variables|Default|GetCurrentLife) (Variables|Default|GetMaxLife))
  (if (<= (Variables|Default|GetCurrentLife) 0.0)
    (Actor|DestroyActor)))

(fn ConstructionScript)