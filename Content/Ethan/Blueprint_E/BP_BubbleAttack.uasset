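; BP_BubbleAttack is a bubble projectile that kills BP_Ennemie actors on contact.
; On BeginPlay it applies a physics impulse to its Sphere along player pawn 0's forward vector, scaled by ImpulseForce, then destroys itself after a short delay.
; A Sphere hit destroys the other actor outright if it is a BP_Ennemie; the bubble itself survives the hit until its timer ends.
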(event OnComponentHit(Sphere)
  (params (HitComponent :type Primitive%20Component%20Object%20Reference) (OtherActor :type Actor%20Object%20Reference) (OtherComp :type Primitive%20Component%20Object%20Reference) (NormalImpulse :type Vector :default "0, 0, 0") (Hit :type Hit%20Result%20Structure%20%28by%20ref%29))
  (bind _asbp_ennemie (Utilities|Casting|CastToBP_Ennemie OtherActor))
  (Actor|DestroyActor _asbp_ennemie))

(event EventBeginPlay
  (Physics|AddImpulse (Variables|Default|GetSphere) (* (Transformation|GetActorForwardVector (Game|Player|GetPlayerPawn 0)) (Variables|Default|GetImpulse%20Force)) "None" false)
  (Utilities|FlowControl|Delay 3.0)
  (Actor|DestroyActor))

(fn ConstructionScript)