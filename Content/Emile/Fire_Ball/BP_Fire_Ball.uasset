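; BP_Fire_Ball is a physics-driven fireball projectile, launched by an impulse on spawn and destroyed after three seconds.
; Tick spawns a new flame effect at its location every frame as it flies.
; Its first hit on a "RockSolid"-tagged actor spawns an explosion and an FS_FireBallForce actor.
; That hit also damages a BP_Tower or BP_Ennemie, hitting enemies harder, then removes the fireball.
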(event OnComponentHit(Sphere)
  (params (HitComponent :type Primitive%20Component%20Object%20Reference) (OtherActor :type Actor%20Object%20Reference) (OtherComp :type Primitive%20Component%20Object%20Reference) (NormalImpulse :type Vector :default "0, 0, 0") (Hit :type Hit%20Result%20Structure%20%28by%20ref%29))
  (bind _outactors (Actor|GetAllActorswithTag "RockSolid"))
  (bind _output_get (Variables|Default|SetNbEnnemi _outactors))
  (for _array_element _output_get
    (if (== OtherActor _array_element)
      (if (not (Variables|Default|GetExplosion))
        (Niagara|SpawnSystematLocation "/Game/Emile/Fire_Ball/P_Explosion.P_Explosion" (Transformation|GetActorLocation) (Transformation|GetActorRotation))
        (CallFunction|ForceProjectile)
        (Variables|Default|SetExplosion true)
        (bind _asbp_tower (Utilities|Casting|CastToBP_Tower OtherActor)
          (:then
            (Variables|/Game/ContentManu/Blueprint/BP_Tower.BP_Tower_C|SetCurrentLife _asbp_tower (- (Variables|/Game/ContentManu/Blueprint/BP_Tower.BP_Tower_C|GetCurrentLife _asbp_tower) 25.0)))
          (:CastFailed
            (bind _asbp_ennemie (Utilities|Casting|CastToBP_Ennemie OtherActor))
            (Variables|/Game/ContentManu/Blueprint/BP_Ennemie.BP_Ennemie_C|SetCurrentLife _asbp_ennemie (- (Variables|/Game/ContentManu/Blueprint/BP_Ennemie.BP_Ennemie_C|GetCurrentLife _asbp_ennemie) 5e+01))))
        (Utilities|FlowControl|Delay 0.01)
        (Actor|DestroyActor)))))

(event Custom|Force_Projectile
  (Utilities|FlowControl|DoOnce false
    (:Completed
      (Game|SpawnActorfromClass "/Game/Emile/Fire_Ball/FS_FireBallForce.FS_FireBallForce_C" (Math|Transform|MakeTransform (Transformation|GetWorldLocation (Variables|Default|GetSphere)) "0, 0, 0" "5.000000,5.000000,5.000000") "Undefined" "MultiplyWithRoot" 0 0))))

(event EventBeginPlay
  (Physics|AddImpulse (Variables|Default|GetSphere) (Variables|Default|GetImpulse%20force) "None" false)
  (Variables|Default|SetExplosion false)
  (Utilities|FlowControl|Delay 3.0)
  (Actor|DestroyActor))

(event Collision|EventActorBeginOverlap
  (params (OtherActor :type Actor%20Object%20Reference)))

(event EventTick
  (params (DeltaSeconds :type Float%20%28single-precision%29))
  (Niagara|SpawnSystematLocation "/Game/Emile/Fire_Ball/P_FlametThrower.P_FlametThrower" (Transformation|GetActorLocation) (Transformation|GetActorRotation)))

(fn ConstructionScript)