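; Mage character Blueprint that casts a fireball with the left mouse button while rooted in place.
; Press and release share one branch on an Attack flag: the first spawns a magic circle underfoot and deactivates movement.
; The next waits a second, spawns BP_Fire_Ball offset along the Shoot component's forward vector with capsule-forward impulse, then removes the circle and restores movement.
; Force scales both spawn offset and impulse.
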(event EventBeginPlay
  (|CallParentFunction))

(event Collision|EventActorBeginOverlap
  (params (OtherActor :type Actor%20Object%20Reference))
  (|CallParentFunction OtherActor) ; This node is disabled and will not be called.\nDrag off pins to build functionality.
)

(event EventTick
  (params (DeltaSeconds :type Float%20%28single-precision%29))
  (|CallParentFunction DeltaSeconds) ; This node is disabled and will not be called.\nDrag off pins to build functionality.
)

(event Input|MouseEvents|LeftMouseButton
  (params (Key :type Key%20Structure :default "None"))
  (bind _returnvalue (Transformation|GetActorTransform))
  (:Pressed
    (if (== (Variables|Default|GetAttack) false) :!label _label
      (bind _returnvalue_2 (Niagara|SpawnSystematLocation "/Game/Emile/P_Magic_Circle.P_Magic_Circle" (+ "0.000000,0.000000,-90.000000" (.location _returnvalue))))
      (Variables|Default|SetAttack true)
      (Components|Activation|Deactivate (Variables|Character|GetCharacterMovement))
      (else
        (Utilities|FlowControl|Delay 1.0)
        (Game|SpawnActorfromClass "/Game/Emile/Fire_Ball/BP_Fire_Ball.BP_Fire_Ball_C" (Math|Transform|MakeTransform (+ (.location _returnvalue) (* (Math|Vector|GetForwardVector (Variables|Default|GetShoot)) (Variables|Default|GetForce))) (.rotation _returnvalue) "1.000000,1.000000,1.000000") "Undefined" "MultiplyWithRoot" 0 (* (Math|Vector|GetForwardVector (Variables|Default|GetCapsuleComponent)) (Variables|Default|GetForce)) 0)
        (Variables|Default|SetAttack false)
        (Components|Activation|Activate (Variables|Character|GetCharacterMovement) false)
        (Components|DestroyComponent _returnvalue_2))))
  (:Released
    (goto _label)))

(fn ConstructionScript
  (|CallParentFunction))