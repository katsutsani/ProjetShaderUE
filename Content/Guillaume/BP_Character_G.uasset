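; BP_Character_G is a character Blueprint with a test primary attack that spawns a ribbon Niagara effect on its weapon.
; Pressing PrimaryAttack prints a debug "Hello" and attaches NS_Ribbon to the Weapon component.
; The effect spawns with auto-activate off and is never activated here, and receives the weapon's world transform as a relative offset.
; BeginPlay and the construction script only call their parents.
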(event EventBeginPlay
  (|CallParentFunction))

(event Collision|EventActorBeginOverlap
  (params (OtherActor :type Actor%20Object%20Reference))
  (|CallParentFunction OtherActor) ; This node is disabled and will not be called.\nDrag off pins to build functionality.
)

(event EventTick
  (params (DeltaSeconds :type Float%20%28single-precision%29))
  (|CallParentFunction DeltaSeconds) ; This node is disabled and will not be called.\nDrag off pins to build functionality.
)

(event Input|ActionEvents|InputActionPrimaryAttack
  (params (Key :type Key%20Structure :default "None"))
  (bind _weapon (Variables|Default|GetWeapon))
  (:Pressed
    (Development|PrintString "Hello")
    (Niagara|SpawnSystemAttached "/Game/Guillaume/NS_Ribbon.NS_Ribbon" _weapon "None" (Transformation|GetWorldLocation _weapon) (Transformation|GetWorldRotation _weapon) "KeepRelativeOffset" false false)))

(fn ConstructionScript
  (|CallParentFunction))