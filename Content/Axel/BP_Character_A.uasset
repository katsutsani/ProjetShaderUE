(event EventBeginPlay
  (Components|Activation|Deactivate (Variables|Default|GetShield_nul)))

(event Input|KeyboardEvents|O
  (params (Key :type Key%20Structure))
  (bind _shield (Variables|Default|GetShield))
  (:Pressed
    (bind _returnvalue (Rendering|Material|CreateDynamicMaterialInstance _shield 0 (Rendering|Material|GetMaterial _shield 0) "None" :!class /Script/Engine.PrimitiveComponent))
    (bind _newtrack_0 (Timeline|Timeline_1 Play)
      (:Update
        (Rendering|Material|SetScalarParameterValue _returnvalue "DissolveAmount" _newtrack_0 :!class /Script/Engine.MaterialInstanceDynamic))
      (:Finished
        (Utilities|FlowControl|Delay 5.0)
        (Rendering|Material|SetScalarParameterValue _returnvalue "Destroy" 1.0 :!class /Script/Engine.MaterialInstanceDynamic)
        (bind _newtrack_0_2 (Timeline|Timeline_2 PlayFromStart)
          (:Update
            (Rendering|Material|SetScalarParameterValue _returnvalue "TimeSpeed" _newtrack_0_2 :!class /Script/Engine.MaterialInstanceDynamic))
          (:Finished
            (bind _newtrack_0_3 (Timeline|Timeline_3 PlayFromStart)
              (:Update
                (Rendering|Material|SetScalarParameterValue _returnvalue "DissolveAmount" _newtrack_0_3 :!class /Script/Engine.MaterialInstanceDynamic)))))))))

(event Input|KeyboardEvents|I
  (params (Key :type Key%20Structure))
  (bind _shield_nul (Variables|Default|GetShield_nul))
  (:Pressed
    (Utilities|FlowControl|FlipFlop
      (:A
        (Components|Activation|Activate _shield_nul false)
        (bind _newtrack_0 (Timeline|Timeline Play)
          (:Update
            (Transformation|SetWorldScale3D (Variables|Default|GetShield_nul) (Math|Conversions|ToVector(Float) _newtrack_0)))))
      (:B
        (Components|Activation|Deactivate _shield_nul)
        (Timeline|Timeline Reverse)))))

(event Input|KeyboardEvents|U
  (params (Key :type Key%20Structure))
  (bind _curvenoise (Variables|Default|GetCurveNoise))
  (:Pressed
    (Utilities|FlowControl|FlipFlop
      (:A
        (Components|Activation|Activate _curvenoise false)
        (bind _newtrack_0 (Timeline|Timeline_0 Play)
          (:Update
            (Transformation|SetWorldScale3D (Variables|Default|GetCurveNoise) (Math|Conversions|ToVector(Float) _newtrack_0)))))
      (:B
        (Components|Activation|Deactivate _curvenoise)
        (Timeline|Timeline_0 Reverse)))))

(fn ConstructionScript
  (|CallParentFunction))