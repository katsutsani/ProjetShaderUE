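; BP_HexaShield is a shield effect actor that runs a timed dissolve and destroy sequence on its Sphere's material.
; After a short delay on BeginPlay, it creates a dynamic material instance and a timeline drives DissolveAmount.
; After a hold, it sets the Destroy parameter, then chained timelines animate TimeSpeed and DissolveAmount again.
; The sequence is purely visual, with no collision, damage or actor destruction logic.
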(event EventBeginPlay
  (bind _sphere (Variables|Default|GetSphere))
  (Utilities|FlowControl|Delay 2.0)
  (bind _returnvalue (Rendering|Material|CreateDynamicMaterialInstance _sphere 0 (Rendering|Material|GetMaterial _sphere 0) "None" :!class /Script/Engine.PrimitiveComponent))
  (bind _newtrack_0 (Timeline|Timeline Play)
    (:Update
      (Rendering|Material|SetScalarParameterValue _returnvalue "DissolveAmount" _newtrack_0 :!class /Script/Engine.MaterialInstanceDynamic))
    (:Finished
      (Utilities|FlowControl|Delay 5.0)
      (Rendering|Material|SetScalarParameterValue _returnvalue "Destroy" 1.0 :!class /Script/Engine.MaterialInstanceDynamic)
      (bind _newtrack_0_2 (Timeline|Timeline_0 PlayFromStart)
        (:Update
          (Rendering|Material|SetScalarParameterValue _returnvalue "TimeSpeed" _newtrack_0_2 :!class /Script/Engine.MaterialInstanceDynamic))
        (:Finished
          (bind _newtrack_0_3 (Timeline|Timeline_1 PlayFromStart)
            (:Update
              (Rendering|Material|SetScalarParameterValue _returnvalue "DissolveAmount" _newtrack_0_3 :!class /Script/Engine.MaterialInstanceDynamic))))))))

(fn ConstructionScript)