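; Player controller that lets the player cycle control among all BP_Character1 instances in the level, starting with the first one found.
; The ToogleWeaponWheel input advances a wrapping index; PossesNewPlayer saves control rotation, waits a tick, possesses the next character, restores rotation and calls update hooks around the swap.
; Movement and yaw input are handled here.
; A weapon wheel widget is created, but its display logic is disconnected.
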(event Custom|PossesNewPlayer
  (params (NewCharacter :type BP%20Character%201%20Object%20Reference))
  (bind _output_get (Variables|Default|SetNewPlayer NewCharacter))
  (Default|UpdateCharacterBeforeUnpossess (Variables|Default|GetActualPlayer))
  (CallFunction|GetControlRot)
  (Utilities|FlowControl|DelayUntilNextTick)
  (Pawn|Possess _output_get)
  (Input|EnableInput self)
  (Default|UpdateCharAfterPosses NewCharacter (Variables|Default|GetActualPlayer))
  (Pawn|SetControlRotation (Variables|Default|GetcontrolRot))
  (Variables|Default|SetActualPlayer _output_get))

(event EventBeginPlay
  (bind _returnvalue (UserInterface|CreateWidget "/Game/Guillaume/WDG_WeaponWheel.WDG_WeaponWheel_C"))
  (Variables|Default|SetWidget _returnvalue)
  (bind _outactors (Actor|GetAllActorsOfClass "/Game/BP_Character1.BP_Character1_C"))
  (bind _output_get (Variables|Default|SetAllCharacter _outactors))
  (Variables|Default|SetActualPlayer (Utilities|Array|Get(acopy) _output_get))
  (CallFunction|PossesNewPlayer (Utilities|Array|Get(acopy) _output_get)))

(event Input|ActionEvents|InputActionToogleWeaponWheel
  (params (Key :type Key%20Structure :default "None"))
  (:Pressed
    (bind _output_get (Variables|Default|Setindex (+ (Variables|Default|Getindex) 1)))
    (if (> _output_get (- (Utilities|Array|Length (Variables|Default|GetAllCharacter)) 1))
      (Variables|Default|Setindex 0))
    (CallFunction|PossesNewPlayer (Utilities|Array|Get(acopy) (Variables|Default|GetAllCharacter) (Variables|Default|Getindex)))))

(event Input|AxisEvents|InputAxisMoveForward
  (params (AxisValue :type Float%20%28single-precision%29))
  (Pawn|Input|AddMovementInput (Variables|Default|GetActualPlayer) (Transformation|GetActorForwardVector) AxisValue false))

(event Input|AxisEvents|InputAxisMoveRight
  (params (AxisValue :type Float%20%28single-precision%29))
  (Pawn|Input|AddMovementInput (Variables|Default|GetActualPlayer) (Transformation|GetActorRightVector) AxisValue false))

(event Input|AxisEvents|InputAxisTurn
  (params (AxisValue :type Float%20%28single-precision%29))
  (Class|PlayerController|AddYawInput AxisValue))

(fn ConstructionScript)

(fn GetControlRot
  (Variables|Default|SetcontrolRot (Pawn|GetControlRotation (Variables|Default|GetActualPlayer) :!class /Script/Engine.Pawn)))